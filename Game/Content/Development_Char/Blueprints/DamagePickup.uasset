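; DamagePickup is a side-scroller hazard pickup that hurts the character who touches it, then destroys itself.
; On overlap it casts to SideScrollerCharacter, lowers one enum-selected stat via an animated ModifyStat call and calls DamagePlayer.
; If that stat's current value reaches zero, it calls Death on player character 0 and prints a death message.
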(event `self.ReceiveActorBeginOverlap`
  (params (OtherActor :type "Actor Object Reference"))
  (bind _asside_scroller_character (cast `/Game/Development_Char/Blueprints/SideScrollerCharacter` OtherActor))
  (`/Game/Development_Char/Blueprints/SideScrollerCharacter.ModifyStat` _asside_scroller_character "NewEnumerator1" -20 true)
  (`/Game/Development_Char/Blueprints/SideScrollerCharacter.DamagePlayer` _asside_scroller_character)
  (if (== (`.CurrentValue_6_A155D8674599DC266737D69DB0929846` (break `/Game/Development_Char/SkillSystem/Structures/s_StatData` (`/Game/Development_Char/Blueprints/SideScrollerCharacter.GetStat` _asside_scroller_character "NewEnumerator1"))) 0)
    (bind _asside_scroller_character_2 (cast `/Game/Development_Char/Blueprints/SideScrollerCharacter` (`GameplayStatics.GetPlayerCharacter` 0)))
    (`/Game/Development_Char/Blueprints/SideScrollerCharacter.Death` _asside_scroller_character_2)
    (`KismetSystemLibrary.PrintString` "You died!")
    (`self.K2_DestroyActor`)
    (else
      (`self.K2_DestroyActor`))))

(fn `UserConstructionScript`)