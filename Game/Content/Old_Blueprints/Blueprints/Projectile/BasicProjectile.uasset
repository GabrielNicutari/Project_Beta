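; BasicProjectile is a player projectile Blueprint that damages Master_Enemy actors on overlap.
; An overlap sends a fixed damage message, spawns an explosion emitter at the enemy's HitArrow and plays a 2D sound.
; It then flags ProjectileHit on the player's SideScrollerCharacter and destroys itself.
; Blocking hits only apply a velocity-based impulse to its own collision component, scaled to zero, so they have no effect.
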(event `self.ReceiveHit`
  (params (MyComp :type "PrimitiveComponent Object Reference") (Other :type "Actor Object Reference") (OtherComp :type "PrimitiveComponent Object Reference") (bSelfMoved :type Boolean) (HitLocation :type "Vector Structure") (HitNormal :type "Vector Structure") (NormalImpulse :type "Vector Structure") (Hit :type "HitResult Structure (by ref)"))
  (`PrimitiveComponent.AddImpulseAtLocation` (`self.ProjectileCollision`) (* (`self.GetVelocity`) 0.0) (`self.K2_GetActorLocation`) "None"))

(event `self.ReceiveActorBeginOverlap`
  (params (OtherActor :type "Actor Object Reference"))
  (bind _asmaster_enemy (cast `/Game/Old_Blueprints/SkillSystem/AI/Enemies/Master_Enemy` OtherActor))
  (message `/Game/Old_Blueprints/SkillSystem/Interfaces/i_Damageable.OnReceiveDamage` _asmaster_enemy 5.0 null null)
  (`GameplayStatics.SpawnEmitterAtLocation` "/Game/Old_Blueprints/Blueprints/Projectile/P_Expl.P_Expl" (`SceneComponent.K2_GetComponentLocation` (`/Game/Old_Blueprints/SkillSystem/AI/Enemies/Master_Enemy.HitArrow` _asmaster_enemy)))
  (`GameplayStatics.SpawnSound2D` "/Game/Old_Blueprints/Sounds/SFX/Sub_Sonic_06.Sub_Sonic_06" 0.2)
  (bind _asside_scroller_character (cast `/Game/Old_Blueprints/Blueprints/SideScrollerCharacter` (`GameplayStatics.GetPlayerCharacter` 0)))
  (set `/Game/Old_Blueprints/Blueprints/SideScrollerCharacter.ProjectileHit` true _asside_scroller_character)
  (`self.K2_DestroyActor`))

(fn `UserConstructionScript`)