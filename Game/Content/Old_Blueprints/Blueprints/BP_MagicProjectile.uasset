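; BP_MagicProjectile is the Cursed Touch magic projectile, which damages enemies and rewards the player on a hit.
; On overlapping a Master_Enemy, it sends a damage message and spawns an explosion at the enemy's HitArrow.
; It then raises a stat on the SideScrollerCharacter, attaches a health-pickup effect, plays a sound and sets CursedTouchHit before destroying itself.
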(event `self.ReceiveActorBeginOverlap`
  (params (OtherActor :type "Actor Object Reference"))
  (bind _asmaster_enemy (cast `/Game/Old_Blueprints/SkillSystem/AI/Enemies/Master_Enemy` OtherActor))
  (message `/Game/Old_Blueprints/SkillSystem/Interfaces/i_Damageable.OnReceiveDamage` _asmaster_enemy 50.0 null null)
  (`GameplayStatics.SpawnEmitterAtLocation` "/Game/Old_Blueprints/Particles/FX_Ability/Summon/CursedTouch_Explosion.CursedTouch_Explosion" (`SceneComponent.K2_GetComponentLocation` (`/Game/Old_Blueprints/SkillSystem/AI/Enemies/Master_Enemy.HitArrow` _asmaster_enemy)))
  (bind _asside_scroller_character (cast `/Game/Old_Blueprints/Blueprints/SideScrollerCharacter` (`GameplayStatics.GetPlayerCharacter` 0)))
  (`/Game/Old_Blueprints/Blueprints/SideScrollerCharacter.ModifyStat` _asside_scroller_character "NewEnumerator1" 50 true)
  (`GameplayStatics.SpawnEmitterAttached` "/Game/Old_Blueprints/Particles/FX_Ability/Heal/P_Health_Pickup_01.P_Health_Pickup_01" (`Character.Mesh` _asside_scroller_character))
  (`GameplayStatics.SpawnSound2D` "/Game/Old_Blueprints/Sounds/Abilites/CursedTouch/Dramatic_Hit_Eerie_07.Dramatic_Hit_Eerie_07")
  (set `/Game/Old_Blueprints/Blueprints/SideScrollerCharacter.CursedTouchHit` true _asside_scroller_character)
  (`self.K2_DestroyActor`))

(fn `UserConstructionScript`)